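; Counter blueprint that tallies destroyed actors, noted as CounterAgents, and changes the scene once four are gone.
; A destroyed-event binding made at BeginPlay increments Counter.
; At four it hides two lights, destroys two chairs, a statue and a table, then spawns a TriggerCapsule_Blueprint at a fixed location and passes it the Floor reference.
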(event Custom|OnDestroyed_Event
  (params (DestroyedActor :type Actor%20Object%20Reference))
  ;[1 1 1] Add to Counter when CounterAgents are destroyed
  (bind _output_get (Variables|Default|SetCounter (+ (Variables|Default|GetCounter) 1)))
  (if (== _output_get 4)
    (Rendering|SetActorHiddenInGame (Variables|Default|GetLight1) true)
    (Actor|DestroyActor (Variables|Default|GetChair1))
    (bind _returnvalue (Game|SpawnActorfromClass "/Game/2DWorldAssets/Blueprints/TriggerCapsule_Blueprint.TriggerCapsule_Blueprint_C" (Math|Conversions|ToTransform(Vector) "-750.000000,1900.000000,2.000000") "AlwaysSpawn" 0 0))
    (bind _astrigger_capsule_blueprint (Utilities|Casting|CastToTriggerCapsule_Blueprint _returnvalue))
    (Variables|/Game/2DWorldAssets/Blueprints/TriggerCapsule_Blueprint.TriggerCapsule_Blueprint_C|SetFloor _astrigger_capsule_blueprint (Variables|Default|GetFloor))))

(event EventBeginPlay
  ;[1 1 1] Add to Counter when CounterAgents are destroyed
  (Game|AssignOnDestroyed (delegate Custom|OnDestroyed_Event)))

(fn ConstructionScript)